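; Grid obstacle actor that occupies a tile and can be destroyed on impact.
; On BeginPlay it takes the grid system from its owner, clears its tile reference and scales itself relative to 70% of the tile width.
; OnImpact, given a valid tile, unblocks it, swaps the cube material, then destroys the actor after a brief delay.
; A separate OnPoints event spawns a points actor at the tile, carrying the destroy score.
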(event EventBeginPlay
  (bind _aso_grid_system (Utilities|Casting|CastTooGridSystem (Components|GetOwner)))
  (Variables|Default|SetoGridSystem _aso_grid_system)
  (bind _output_get (Variables|Default|SetoGridTileReference 0))
  (Utilities|IsValid _output_get
    (:Is%20Valid
      _)
    (:Is%20Not%20Valid
      _))
  (CallFunction|ScaletoGrid))

(event Collision|EventActorBeginOverlap
  (params (OtherActor :type Actor%20Object%20Reference)))

(event EventTick
  (params (DeltaSeconds :type Float%20%28single-precision%29)))

(event EventOnPoints
  (Game|SpawnActorfromClass "/Game/Widgets/aPointsSpawn.aPointsSpawn_C" (Transformation|GetActorTransform (Variables|Default|GetoGridTileReference)) "Undefined" 0 (Variables|Default|GetiDestroyPoints) 0))

(event EventOnImpact
  (bind _ogridtilereference (Variables|Default|GetoGridTileReference))
  (Utilities|IsValid _ogridtilereference
    (:Is%20Valid
      (Variables|/Game/GameActors/Blueprints/Grid/oGridTile.oGridTile_C|SetoActorOnTile _ogridtilereference 0)
      (Variables|/Game/GameActors/Blueprints/Grid/oGridTile.oGridTile_C|SetfIsBlocking _ogridtilereference false)
      (Rendering|Material|SetMaterial (Variables|Default|Getcube) 0 "/Engine/EngineMaterials/CubeMaterial.CubeMaterial")
      (Utilities|FlowControl|RetriggerableDelay 0.1)
      (Actor|DestroyActor))))

(fn ConstructionScript)

(fn ScaletoGrid
  (Transformation|SetActorScale3D (* (Transformation|GetActorScale3D) (/ (* (* (Variables|/Game/GameActors/Blueprints/Grid/oGridSystem.oGridSystem_C|GetfTileHalfExtent (Variables|Default|GetoGridSystem)) 2.0) 0.7) 1e+02))))