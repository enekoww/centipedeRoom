(event EventTick
  (params (DeltaSeconds :type Float%20%28single-precision%29))
  (bind _cube (Variables|Components|GetCube))
  (if (Variables|OwnerBooleans|GetfIsBlocking)
    (Rendering|SetVisibility _cube true false)
    (else
      (Rendering|SetVisibility _cube false false))))

(event Collision|EventActorBeginOverlap
  (params (OtherActor :type Actor%20Object%20Reference)))

(event EventOnImpact)

(event EventBeginPlay
  (bind _aso_grid_system (Utilities|Casting|CastTooGridSystem (Components|GetOwner)))
  (Variables|Default|SetoGridSystem _aso_grid_system)
  (Variables|Default|SetvGridWorldLocation (Transformation|GetActorLocation))
  (bind _asgm_console_room (Utilities|Casting|CastTogmConsoleRoom (Game|GetGameMode)))
  (Variables|Default|SetgmConsoleRoom _asgm_console_room))

(event EventOnKill
  (bind _oobstacle (Variables|Default|GetoObstacle))
  (Default|OnImpact _oobstacle)
  (Default|OnPoints _oobstacle))

(fn ConstructionScript
  (Variables|Default|SetfBoxSize (Variables|Default|GetfBoxSize)))

(fn MakeBlocking
  (params (CurrentTile :type O%20Grid%20Tile%20Object%20Reference))
  (Utilities|IsValid CurrentTile
    (:Is%20Valid
      (Variables|OwnerBooleans|SetfIsBlocking true)
      (bind _returnvalue (Game|SpawnActorfromClass "/Game/GameActors/Blueprints/Grid/Obstacle.Obstacle_C" (Transformation|GetActorTransform) "Undefined" (Variables|Default|GetoGridSystem) self 0))
      (bind _output_get (Variables|Default|SetoObstacle _returnvalue))
      (Utilities|IsValid _output_get
        (:Is%20Valid
          (Variables|/Game/GameActors/Blueprints/Grid/Obstacle.Obstacle_C|SetoGridTileReference _returnvalue CurrentTile)
          (Variables|Default|SetoActorOnTile _returnvalue)
          (return _returnvalue))
        (:Is%20Not%20Valid
          (Development|PrintString "not valid opn spawbn"))))))

(fn MakeNonBlocking
  (Variables|OwnerBooleans|SetfIsBlocking false)
  (Rendering|SetVisibility (Variables|Components|GetCube) false false))

(fn MakeBoundary
  (params (CurrentTile :type O%20Grid%20Tile%20Object%20Reference))
  (Variables|OwnerBooleans|SetfIsBlocking true)
  (bind _returnvalue (Game|SpawnActorfromClass "/Game/GameActors/Blueprints/Grid/Bounding.Bounding_C" (Transformation|GetActorTransform) "Undefined" (Variables|Default|GetoGridSystem) 0 0))
  (bind _output_get (Variables|Default|SetoObstacle _returnvalue))
  (Variables|/Game/GameActors/Blueprints/Grid/Obstacle.Obstacle_C|SetoGridTileReference _returnvalue CurrentTile)
  (Variables|OwnerBooleans|SetbIsBoundary true)
  (return _output_get))

(fn GivePoints
  (Game|SpawnActorfromClass "/Game/Widgets/aPointsSpawn.aPointsSpawn_C" (Transformation|GetActorTransform) "Undefined" 0 (Variables|Default|GetiPointsForDestroying) 0))

(fn MakeBlockingSpecial
  (params (CurrentTile :type O%20Grid%20Tile%20Object%20Reference))
  (Utilities|IsValid CurrentTile
    (:Is%20Valid
      (Variables|OwnerBooleans|SetfIsBlocking true)
      (bind _returnvalue (Game|SpawnActorfromClass "/Game/GameActors/Blueprints/Grid/oBarrel.oBarrel_C" (Transformation|GetActorTransform) "Undefined" (Variables|Default|GetoGridSystem) self 0))
      (bind _output_get (Variables|Default|SetoObstacle _returnvalue))
      (Utilities|IsValid _output_get
        (:Is%20Valid
          (Variables|/Game/GameActors/Blueprints/Grid/Obstacle.Obstacle_C|SetoGridTileReference _returnvalue CurrentTile)
          (Variables|Default|SetoActorOnTile _returnvalue)
          (return _returnvalue))
        (:Is%20Not%20Valid
          (Development|PrintString "not valid opn spawbn"))))))