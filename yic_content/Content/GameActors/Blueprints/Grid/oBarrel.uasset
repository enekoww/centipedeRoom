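; Barrel grid actor that, on impact, kills nearby tiles, frees its own tile, swaps its material and destroys itself after a brief delay.
; DestroySurroundings looks up tiles in the grid system's map and calls OnKill, looping each axis from one below the barrel's position to a fixed index 2, not a relative offset.
; A separate OnPoints event spawns a points actor at the tile, carrying the barrel's destroy score.
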(event EventBeginPlay
  (|CallParentFunction) ; This node is disabled and will not be called.\nDrag off pins to build functionality.
)

(event Collision|EventActorBeginOverlap
  (params (OtherActor :type Actor%20Object%20Reference)))

(event EventTick
  (params (DeltaSeconds :type Float%20%28single-precision%29))
  (|CallParentFunction DeltaSeconds) ; This node is disabled and will not be called.\nDrag off pins to build functionality.
)

(event EventOnPoints
  (Game|SpawnActorfromClass "/Game/Widgets/aPointsSpawn.aPointsSpawn_C" (Transformation|GetActorTransform (Variables|Default|GetoGridTileReference)) "Undefined" 0 (Variables|Default|GetiDestroyPoints) 0))

(event EventOnImpact
  (bind _ogridtilereference (Variables|Default|GetoGridTileReference))
  (Utilities|IsValid _ogridtilereference
    (:Is%20Valid
      (CallFunction|DestroySurroundings)
      (Variables|/Game/GameActors/Blueprints/Grid/oGridTile.oGridTile_C|SetoActorOnTile _ogridtilereference 0)
      (Variables|/Game/GameActors/Blueprints/Grid/oGridTile.oGridTile_C|SetfIsBlocking _ogridtilereference false)
      (Rendering|Material|SetMaterial (Variables|Default|Getcube) 0 "/Engine/EngineMaterials/CubeMaterial.CubeMaterial")
      (Utilities|FlowControl|RetriggerableDelay 0.1)
      (Actor|DestroyActor))))

(fn ConstructionScript
  (|CallParentFunction))

(fn DestroySurroundings
  (bind _ogridtilereference (Variables|Default|GetoGridTileReference))
  (bind _v2dgridposition (Variables|/Game/GameActors/Blueprints/Grid/oGridTile.oGridTile_C|Getv2dGridPosition _ogridtilereference))
  (bind _returnvalue (- _v2dgridposition "(X=1.000000,Y=1.000000)"))
  (for _index (range (Math|Float|Truncate (.x _returnvalue)) 2)
    (for _index_2 (range (Math|Float|Truncate (.y _returnvalue)) 2)
      (Default|OnKill (.Value (Utilities|Map|Find (Variables|/Game/GameActors/Blueprints/Grid/oGridSystem.oGridSystem_C|GetmGridArray (Variables|Default|GetoGridSystem)) (Math|Vector2D|MakeVector2D (Math|Conversions|ToFloat(Integer) _index) (Math|Conversions|ToFloat(Integer) _index_2))))))))