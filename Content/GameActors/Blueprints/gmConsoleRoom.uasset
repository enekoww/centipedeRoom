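; Game mode for the console room, running a Centipede-style grid game from the cartridge in an in-world console.
; It builds the grid from the cart's seed, spawns centipede, shooter, overseer and an orthographic scene-capture camera, and handles reset, shutdown and maze regeneration.
; Looping timers broadcast separate player, shooter and projectile move pulses, with pause and a temporary dash speed-up.
; The player possesses the centipede while viewing through the first-person character.
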(event Custom|NewGame
  ;[1 1 1] Initialize New Grid and Game
  (Utilities|FlowControl|Sequence
    (:then_0
      (Utilities|FlowControl|DoOnce false
        (:Completed
          (CallFunction|SetNewCamera))))
    (:then_1
      (bind _gridsystem (CallFunction|SpawnGridSystem))
      (Utilities|IsValid _gridsystem
        (:Is%20Valid
          (bind _output_get (Variables|Default|SetoGridSystem _gridsystem))
          (Variables|Default|SetvGridSystemPos (Variables|/Game/GameActors/Blueprints/Grid/oGridSystem.oGridSystem_C|GetvDesiredLocation _output_get))
          (CallFunction|SpawnCentipede)
          (CallFunction|CreateOverseer)
          (CallFunction|SpawnShooter)
          (CallFunction|PossesCentipede)
          (CallFunction|StartPulseEvents))))))

(event Custom|RegenerateGame
  (bind _ogridsystem (Variables|Default|GetoGridSystem))
  ;[1 1 1] Regenerates Maze
  (bind _values (Utilities|Map|Values (Variables|/Game/GameActors/Blueprints/Grid/oGridSystem.oGridSystem_C|GetmGridArray (Variables|Default|GetoGridSystem))))
  (for _array_element _values
    (Default|MakeNonBlocking _array_element)
    (Utilities|IsValid (Variables|/Game/GameActors/Blueprints/Grid/oGridTile.oGridTile_C|GetoObstacle _array_element)
      (:Is%20Valid
        (Actor|DestroyActor (Variables|/Game/GameActors/Blueprints/Grid/oGridTile.oGridTile_C|GetoObstacle _array_element))
        (CallFunction|StopPulseEvents))))
  (Default|RandomObstacleGeneratorStop _ogridsystem)
  (CallFunction|DestroyProjectiles)
  (CallFunction|DestroyEggs)
  (CallFunction|DestroyCentipede)
  (Default|ReconstructGrid _ogridsystem)
  (CallFunction|SpawnCentipede)
  (CallFunction|PossesCentipede)
  (Default|CallSetOverseer (Variables|Default|GetoGameOverseer))
  (CallFunction|StopPulseEvents)
  (Utilities|FlowControl|RetriggerableDelay 4.0)
  (CallFunction|StartPulseEvents))

(event Custom|PausePlayerTimer
  ;[1 0.7417 0.6408 1 30] Custom Ticks
  (Utilities|Time|PauseTimerbyHandle (Variables|Default|GetPlayerTimer))
  (Default|UpdateTrail (Variables|Default|GetoCentipedePawnHead)))

(event Custom|ResumePlayerTimer
  ;[1 0.7417 0.6408 1 30] Custom Ticks
  (Utilities|Time|UnpauseTimerbyHandle (Variables|Default|GetPlayerTimer)))

(event Custom|AcceleratePlayerTimer
  ;[1 0.7417 0.6408 1 30] Custom Ticks
  (Utilities|Time|ClearandInvalidateTimerbyHandle (Variables|Default|GetPlayerTimer))
  (bind _returnvalue (Utilities|Time|SetTimerbyFunctionName 0 "PlayerMovePulse" (/ 1.0 (* (Variables|Default|GetPlayerTicksPerSecond) 3.0)) true))
  (Variables|Default|SetPlayerTimer _returnvalue)
  (Utilities|FlowControl|Delay 0.5)
  (CallFunction|ResetPlayerTimer))

(event Custom|ResetPlayerTimer
  ;[1 0.7417 0.6408 1 30] Custom Ticks
  (bind _returnvalue (Utilities|Time|SetTimerbyFunctionName 0 "PlayerMovePulse" (/ 1.0 (Variables|Default|GetPlayerTicksPerSecond)) true))
  (Variables|Default|SetPlayerTimer _returnvalue)
  (Variables|/Game/GameActors/Blueprints/Characters/Player/oCentipedeChain.oCentipedeChain_C|SetbIsDashing (Variables|Default|GetoCentipedePawnHead) false))

(event Custom|TurnOffConsole
  (bind _ogridsystem (Variables|Default|GetoGridSystem))
  ;[1 1 1] Destroy Current Game
  (Utilities|IsValid _ogridsystem
    (:Is%20Valid
      (Default|AutoDestroy _ogridsystem)
      (Actor|DestroyActor _ogridsystem))))

(event Custom|StopPulseEvents
  ;[1 0.7417 0.6408 1 30] Custom Ticks
  (Utilities|Time|ClearandInvalidateTimerbyHandle (stale Custom|StartPulseEvents _returnvalue))
  (Utilities|Time|ClearandInvalidateTimerbyHandle (stale Custom|StartPulseEvents _returnvalue_2))
  (Utilities|Time|ClearandInvalidateTimerbyHandle (stale Custom|StartPulseEvents _returnvalue_3)))

(event Custom|StartPulseEvents
  ;[1 0.7417 0.6408 1 30] Custom Ticks
  (bind _returnvalue (Utilities|Time|SetTimerbyFunctionName 0 "PlayerMovePulse" (/ 1.0 (Variables|Default|GetPlayerTicksPerSecond)) true))
  (Variables|Default|SetPlayerTimer _returnvalue)
  (bind _returnvalue_2 (Utilities|Time|SetTimerbyFunctionName 0 "ShooterMovePulse" (/ 1.0 (Variables|Default|GetShooterTicksPerSecond)) true))
  (Variables|Default|SetShooterTimer _returnvalue_2)
  (bind _returnvalue_3 (Utilities|Time|SetTimerbyFunctionName 0 "ProjectileMovePulse" (/ 1.0 (Variables|Default|GetProjectilesTicksPerSecond_0)) true))
  (Variables|Default|SetProjectileTimer _returnvalue_3))

(event Custom|Reset%20All
  (bind _ogridsystem (Variables|Default|GetoGridSystem))
  ;[1 1 1] ResetsAll New game Created
  (Utilities|IsValid _ogridsystem
    (:Is%20Valid
      (Default|AutoDestroy _ogridsystem)
      (Actor|DestroyActor (Variables|Default|GetoGameOverseer))
      (Actor|DestroyActor _ogridsystem)
      (CallFunction|StopPulseEvents))
    (:Is%20Not%20Valid
      _))
  (CallFunction|NewGame))

(event EventBeginPlay
  ;[1 1 1] Begin Play
  (bind _outactors (Actor|GetAllActorsOfClass "/Game/GameActors/Blueprints/FirstPersonCharacter.FirstPersonCharacter_C"))
  (Variables|Default|SetoPlayerPawn (Utilities|Array|Get(acopy) _outactors)))

(fn ConstructionScript)

(fn DestroyProjectiles
  (bind _outactors (Actor|GetAllActorsOfClass "/Game/GameActors/Blueprints/Characters/Enemy/aProjectile.aProjectile_C"))
  (for _array_element _outactors
    (Utilities|IsValid _array_element
      (:Is%20Valid
        (Actor|DestroyActor _array_element)))))

(fn DestroyEggs
  (bind _outactors (Actor|GetAllActorsOfClass "/Game/GameActors/Blueprints/Characters/Player/oEgg.oEgg_C"))
  (for _array_element _outactors
    (Utilities|IsValid _array_element
      (:Is%20Valid
        (Actor|DestroyActor _array_element)))))

(fn SpawnCentipede
  (bind _ogridsystem (Variables|Default|GetoGridSystem))
  (Utilities|Array|Clear (Variables|Default|GetaCentipedeChain))
  (CallFunction|DestroyCentipede)
  (for _index (range 0 (Variables|Default|GetiTailLength))
    (bind _returnvalue (Game|SpawnActorfromClass "/Game/GameActors/Blueprints/Characters/Player/oCentipedeChain.oCentipedeChain_C" (Math|Transform|MakeTransform "0, 0, 0" "0, 0, 0" "1,1,1") "Undefined" _ogridsystem _ogridsystem _index 0))
    (Utilities|Array|Add (Variables|Default|GetaCentipedeChain) _returnvalue)))

(fn SpawnCentipedeHead
  (params (Length :type Integer))
  (bind _ogridsystem (Variables|Default|GetoGridSystem))
  (for _index (range 0 3)
    (Development|PrintString "Hello")
    (bind _returnvalue (Game|SpawnActorfromClass "/Game/GameActors/Blueprints/Characters/Player/oCentipedeChain.oCentipedeChain_C" (Math|Transform|MakeTransform "0, 0, 0" "0, 0, 0" "1,1,1") "Undefined" _ogridsystem _ogridsystem _index 0))
    (Utilities|Array|AddUnique (Variables|Default|GetaCentipedeChain) _returnvalue)
    (return _returnvalue)))

(fn SpawnCentipedeTails
  (params (NumberOfSegments :type Integer) (CentipedeHead :type P%20Centipede%20Head%20Object%20Reference))
  (bind _ogridsystem (Variables|Default|GetoGridSystem))
  (for _index (range 0 (- NumberOfSegments 1))
    (bind _returnvalue (Game|SpawnActorfromClass "/Game/GameActors/Blueprints/Characters/Player/centipedeTail.centipedeTail_C" (Math|Transform|MakeTransform "0, 0, 0" "0, 0, 0" "1,1,1") "Undefined" _ogridsystem CentipedeHead _ogridsystem _index 0))
    (Utilities|Array|Add (Variables|Default|GetaTailChain) _returnvalue)))

(fn SpawnGridSystem
  (bind _oconsole (Variables|Default|GetoConsole))
  (bind _ogamecartin (Variables|/Game/GameActors/Blueprints/Machines/oConsole.oConsole_C|GetoGameCartIn _oconsole))
  (bind _gridseed (Variables|/Game/GameActors/Blueprints/Machines/oGridCartdridge.oGridCartdridge_C|GetGridSeed _ogamecartin))
  (Utilities|IsValid _ogamecartin
    (:Is%20Valid
      (bind _returnvalue (Game|SpawnActorfromClass "/Game/GameActors/Blueprints/Grid/oGridSystem.oGridSystem_C" (Math|Transform|MakeTransform "0.000000, 0,200.000000" "0, 0, 0" "1,1,1") "Undefined" 0 (.xtilecount _gridseed) (.ytilecount _gridseed) "0.000000,0.000000,300.000000" 1e+01 0 (- (Variables|Default|GetCameraLocation) "0, 0,500.000000") (.ablockingpositionarray _gridseed) 0))
      (return _returnvalue))
    (:Is%20Not%20Valid
      (Development|PrintString "No Game Inserted"))))

(fn SpawnShooter
  (bind _returnvalue (Game|SpawnActorfromClass "/Game/GameActors/Blueprints/Characters/Enemy/aShooter.aShooter_C" (Math|Transform|MakeTransform "0, 0, 0" "0,-90.000000, 0" "1,1,1") "Undefined" (Variables|Default|GetoGridSystem) 0))
  (Variables|Default|SetoShooter _returnvalue))

(fn DestroyCentipede
  (bind _outactors (Actor|GetAllActorsOfClass "/Game/GameActors/Blueprints/Characters/Player/oCentipedeChain.oCentipedeChain_C"))
  (for _array_element _outactors
    (Utilities|IsValid _array_element
      (:Is%20Valid
        (Actor|DestroyActor _array_element)))))

(fn SetNewCamera
  (bind _returnvalue (Game|SpawnActorfromClass "/Game/Camera/SceneCaptureCam.SceneCaptureCam_C" (Math|Transform|MakeTransform (Variables|Default|GetCameraLocation) "-90.000000,0.000000,90.000000" "1,1,1") "Undefined" 0 0))
  (Variables|/Script/Engine.SceneCaptureComponent2D|SetProjectionType (Variables|/Script/Engine.SceneCapture2D|GetCaptureComponent2D _returnvalue) "Orthographic")
  (Variables|/Script/Engine.SceneCaptureComponent2D|SetOrthoWidth (Variables|/Script/Engine.SceneCapture2D|GetCaptureComponent2D _returnvalue) 1.1e+03))

(fn PossesCentipede
  (Pawn|Possess (Game|GetPlayerController 0) (Variables|Default|GetoCentipedePawnHead))
  (Game|Player|SetViewTargetwithBlend (Game|GetPlayerController 0) (Variables|Default|GetoPlayerPawn) 0.0 "VTBlend_Linear" 0.0 false))

(fn CreateOverseer
  (bind _returnvalue (Game|SpawnActorfromClass "/Game/Widgets/oGameOverseer.oGameOverseer_C" (Math|Transform|MakeTransform "0, 0, 0" "0, 0, 0" "1,1,1") "Undefined" 0 0))
  (bind _output_get (Variables|Default|SetoGameOverseer _returnvalue))
  (Utilities|Casting|CastTowbpCentipedeInfo (UserInterface|GetUserWidgetObject (Variables|/Game/GameActors/Blueprints/Machines/oDisplay.oDisplay_C|GetPointSystem (Variables|Default|GetoTelevision))))
  (Default|CallSetOverseer _output_get))

(fn PlayerMovePulse
  (Default|CallPlayerMoveSignal))

(fn ShooterMovePulse
  (Default|CallShooterMoveSignal))

(fn ProjectileMovePulse
  (Default|CallProjectilesMoveSignal))

(fn CleanTailChain
  (bind _atailchain (Variables|Default|GetaTailChain))
  (for (_array_element _array_index) _atailchain
    (Utilities|IsValid _array_element
      (:Is%20Not%20Valid
        (Utilities|Array|RemoveIndex _atailchain _array_index)))))