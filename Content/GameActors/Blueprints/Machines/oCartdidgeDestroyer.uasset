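; An interactable machine that destroys the cart the player is holding and reports the result on its text prompt.
; Overlapping its AreaOfInteraction stores the FirstPersonCharacter, toggles the prompt's visibility and starts a looping timer that yaws the text toward the player.
; The OnActivate interface event destroys that player's OCartAtHand if valid.
; Leaving the area clears the timer and player reference, toggles visibility again and resets the prompt text.
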(event OnComponentBeginOverlap(AreaOfInteraction)
  (params (OverlappedComponent :type Primitive%20Component%20Object%20Reference) (OtherActor :type Actor%20Object%20Reference) (OtherComp :type Primitive%20Component%20Object%20Reference) (OtherBodyIndex :type Integer) (bFromSweep :type Boolean) (SweepResult :type Hit%20Result%20Structure%20%28by%20ref%29))
  ;[1 1 1] Billboard on/off on proximity
  (bind _asfirst_person_character (Utilities|Casting|CastToFirstPersonCharacter OtherActor))
  (Variables|Default|SetPlayer _asfirst_person_character)
  (CallFunction|BilboardModeon))

(event OnComponentEndOverlap(AreaOfInteraction)
  (params (OverlappedComponent :type Primitive%20Component%20Object%20Reference) (OtherActor :type Actor%20Object%20Reference) (OtherComp :type Primitive%20Component%20Object%20Reference) (OtherBodyIndex :type Integer))
  ;[1 1 1] Billboard on/off on proximity
  (if (== OtherActor (Variables|Default|GetPlayer))
    (Variables|Default|SetPlayer 0)
    (CallFunction|BilboardModeOff)
    (Rendering|Components|TextRender|SetText (Variables|Default|GetPrompt) (Utilities|Text|MakeLiteralText "Destroy cart [ e ]"))))

(event EventBeginPlay)

(event Collision|EventActorBeginOverlap
  (params (OtherActor :type Actor%20Object%20Reference)))

(event EventTick
  (params (DeltaSeconds :type Float%20%28single-precision%29)))

(event EventOnActivate
  (bind _player (Variables|Default|GetPlayer))
  (bind _ocartathand (Variables|/Game/GameActors/Blueprints/FirstPersonCharacter.FirstPersonCharacter_C|GetoCartAtHand _player))
  ;[1 1 1] Interface call. Destroy cart if payer holding one
  (Utilities|IsValid _ocartathand
    (:Is%20Valid
      (Actor|DestroyActor _ocartathand)
      (Rendering|Components|TextRender|SetText (Variables|Default|GetPrompt) (Utilities|Text|MakeLiteralText "Awsome cart Destroyed")))
    (:Is%20Not%20Valid
      (Rendering|Components|TextRender|SetText (Variables|Default|GetPrompt) (Utilities|Text|MakeLiteralText "You have no cart to destroy")))))

(fn ConstructionScript)

(fn LookatPlayerText
  (Transformation|SetWorldRotation (Variables|Default|GetPrompt) (Math|Rotator|MakeRotator 0.0 0.0 (.yaw (Math|Rotator|FindLookatRotation (Transformation|GetActorLocation) (Transformation|GetActorLocation (Variables|Default|GetPlayer))))) false false))

(fn BilboardModeon
  (bind _returnvalue (Utilities|Time|SetTimerbyFunctionName 0 "LookAtPlayerText" (Utilities|Time|GetWorldDeltaSeconds) true))
  (Variables|Default|SetLookAtTimer _returnvalue)
  (Rendering|ToggleVisibility (Variables|Default|GetPrompt) false))

(fn BilboardModeOff
  (Utilities|Time|ClearandInvalidateTimerbyHandle (Variables|Default|GetLookAtTimer))
  (Rendering|ToggleVisibility (Variables|Default|GetPrompt) false))