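; A grid cartridge the first-person player picks up and drops, carrying a randomly generated obstacle layout and tinted a random color.
; On BeginPlay it randomizes grid size and block density, walls both X edges, then filters interior cells by Y margins and diagonal adjacency.
; Random candidates become blockers, saved with the dimensions in StGridSeed for reconstruction.
; Activation toggles between socket attachment, when the player's hand is empty, and physics-simulated release.
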(event Custom|Generate%20Grid
  (Utilities|FlowControl|Sequence
    (:then_0
      ;[1 0.6531 0.9344] GidSystem Definition
      (for _index (range 0 (- (Variables|Grid|GetiXCellNumber) 1))
        (Variables|Tile|SetiXIndex _index)
        (for _index_2 (range 0 (- (Variables|Grid|GetiYCellNumber) 1))
          (Variables|Tile|SetiYIndex _index_2)
          (if (or (== (Variables|Tile|GetiXIndex) 0) (== (Variables|Tile|GetiXIndex) (- (Variables|Grid|GetiXCellNumber) 1)))
            ;[0.7917 0.8155 1] Define Boundaries
            (Utilities|Array|Add (Variables|GridArrays|GetsTilesFinalBlockingDefinitionVectors) (Math|Vector2D|MakeVector2D (Math|Conversions|ToFloat(Integer) (Variables|Tile|GetiXIndex)) (Math|Conversions|ToFloat(Integer) (Variables|Tile|GetiYIndex))))
            (else
              ;[0.7917 0.8155 1] Get All Blocking Pos Candidates
              (CallFunction|IsObstaclePosValid (Math|Vector2D|MakeVector2D (Math|Conversions|ToFloat(Integer) (Variables|Tile|GetiXIndex)) (Math|Conversions|ToFloat(Integer) (Variables|Tile|GetiYIndex)))))))))
    (:then_1
      ;[1 1 1] Start Putting Obstacles
      (CallFunction|SetPercentageInitialBlocks (Variables|Grid|GetiPercentageOfBlocks))
      (CallFunction|DefineInitialBlockignTiles))
    (:then_2
      ;[1 1 1] Add To Seed For Reconstruction
      (Variables|Default|SetstGridSeed (Utilities|Struct|MakesTileInfo (Variables|GridArrays|GetsTilesFinalBlockingDefinitionVectors) (Variables|Grid|GetiXCellNumber) (Variables|Grid|GetiYCellNumber))))))

(event Custom|CustomEvent)

(event EventBeginPlay
  (Utilities|FlowControl|Sequence
    (:then_0
      ;[1 1 1] Generate grid logic
      (CallFunction|RandomizeInitialVariables)
      (CallFunction|GenerateGrid))
    (:then_1
      ;[1 1 1] Cart visual
      (bind _returnvalue (Rendering|Material|CreateDynamicMaterialInstance (Variables|Default|GetCube) 0 "/Game/GameActors/Blueprints/Machines/Materials/RandomColorMaterial_Cartdridge_Mat_Inst.RandomColorMaterial_Cartdridge_Mat_Inst" "None" :!class /Script/Engine.PrimitiveComponent))
      (Rendering|Material|SetVectorParameterValue _returnvalue "Color" (Utilities|Struct|MakeLinearColor (Math|Random|RandomFloatinRange 0.0 1.0) (Math|Random|RandomFloatinRange 0.0 1.0) (Math|Random|RandomFloatinRange 0.0 1.0) 1.0) :!class /Script/Engine.MaterialInstanceDynamic))))

(event EventOnActivate
  ;[1 1 1] INterface calls to handle First Person Interactions
  (if (Variables|Default|GetbIsHeld)
    (CallFunction|OnDeactivate)
    (else
      (bind _asfirst_person_character (Utilities|Casting|CastToFirstPersonCharacter (Game|Player|GetPlayerPawn 0)))
      (Utilities|IsValid (Variables|/Game/GameActors/Blueprints/FirstPersonCharacter.FirstPersonCharacter_C|GetoCartAtHand _asfirst_person_character)
        (:Is%20Not%20Valid
          (CallFunction|AttachCarttoPlayer _asfirst_person_character))))))

(event EventOnDeactivate
  ;[1 1 1] INterface calls to handle First Person Interactions
  (bind _asfirst_person_character (Utilities|Casting|CastToFirstPersonCharacter (Game|Player|GetPlayerPawn 0)))
  (CallFunction|DettachCartfromPlayer _asfirst_person_character))

(fn ConstructionScript)

(fn IsObstaclePosValid
  (params (CurrentGrid :type Vector%202D%20Structure))
  (bind _output_get (LocalVariables|Set2dvCandidateVector CurrentGrid))
  (bind _valid (CallFunction|ExistsinArray _output_get))
  (if (not _valid)
    (bind _valid_2 (CallFunction|IsMinMaxYPos (LocalVariables|Get2dvCandidateVector) 2 2 (Variables|Grid|GetiYCellNumber)))
    (if (not _valid_2)
      (bind _diagonals (CallFunction|IsDiagonal (LocalVariables|Get2dvCandidateVector)))
      (if (not _diagonals)
        (Utilities|Array|Add (Variables|GridArrays|GetsTilesBlockingCandidates) (LocalVariables|Get2dvCandidateVector))))))

(fn IsMinMaxYPos
  (params (Candidate%20Vector :type Vector%202D%20Structure) (MinY :type Integer) (MaxY :type Integer) (YLength :type Integer))
  (bind _y (Math|Vector2D|BreakVector2D Candidate%20Vector))
  (return (or (<= (Math|Float|Truncate _y) MinY) (>= (Math|Float|Truncate _y) (- YLength MaxY)))))

(fn ExistsinArray
  (params (CandiDateVector :type Vector%202D%20Structure))
  (return (>= (Utilities|Array|FindItem (Variables|GridArrays|GetsTilesFinalBlockingDefinitionVectors) CandiDateVector) 0)))

(fn IsDiagonal
  (params (CandidateVector :type Vector%202D%20Structure))
  (bind _returnvalue (- (.y CandidateVector) 1.0))
  (bind _stilesfinalblockingdefinitionvectors (Variables|GridArrays|GetsTilesFinalBlockingDefinitionVectors))
  ;[1 1 1] No Diagonals
  (return (or (>= (Utilities|Array|FindItem _stilesfinalblockingdefinitionvectors (Math|Vector2D|MakeVector2D (- (.x CandidateVector) 1.0) _returnvalue)) 0) (>= (Utilities|Array|FindItem _stilesfinalblockingdefinitionvectors (Math|Vector2D|MakeVector2D (+ (.x CandidateVector) 1.0) _returnvalue)) 0))))

(fn DefineInitialBlockignTiles
  (bind _stilesblockingcandidates (Variables|GridArrays|GetsTilesBlockingCandidates))
  (bind _returnvalue (Utilities|Array|Length _stilesblockingcandidates))
  (bind _returnvalue_2 (- _returnvalue 1))
  (bind _returnvalue_3 (Math|Random|RandomInteger _returnvalue_2))
  (for _index (range 0 (Variables|Grid|GetiInitialBlocks))
    (Utilities|Array|Add (Variables|GridArrays|GetsTilesFinalBlockingDefinitionVectors) (Utilities|Array|Get(acopy) _stilesblockingcandidates _returnvalue_3))
    (Utilities|Array|RemoveIndex (Variables|GridArrays|GetsTilesBlockingCandidates) _returnvalue_3)))

(fn SetPercentageInitialBlocks
  (params (PercentageOfBlocks :type Float%20%28single-precision%29))
  (Variables|Grid|SetiInitialBlocks (Math|Float|Truncate (* (Variables|Grid|GetiPercentageOfBlocks) (Math|Conversions|ToFloat(Integer) (- (Utilities|Array|Length (Variables|GridArrays|GetsTilesBlockingCandidates)) 1))))))

(fn RandomizeInitialVariables
  (bind _returnvalue (Math|Random|RandomIntegerinRange 25 30))
  (Variables|Grid|SetiXCellNumber _returnvalue)
  (Variables|Grid|SetiYCellNumber (Math|Random|RandomIntegerinRange _returnvalue 40))
  (Variables|Grid|SetiPercentageOfBlocks (Math|Random|RandomFloatinRange 0.03 0.06)))

(fn AttachCarttoPlayer
  (params (Player :type First%20Person%20Character%20Object%20Reference))
  (Transformation|AttachComponentToComponent self (Variables|/Game/GameActors/Blueprints/FirstPersonCharacter.FirstPersonCharacter_C|GetCartdridgeSocket Player) "CartdridgeSocket" "SnapToTarget" "SnapToTarget" "KeepWorld" true)
  (Variables|/Game/GameActors/Blueprints/FirstPersonCharacter.FirstPersonCharacter_C|SetoCartAtHand Player self)
  (Physics|SetSimulatePhysics (Variables|Default|GetCartdidgeColl) false)
  (Variables|Default|SetbIsHeld true))

(fn DettachCartfromPlayer
  (params (Player :type First%20Person%20Character%20Object%20Reference))
  (Variables|/Game/GameActors/Blueprints/FirstPersonCharacter.FirstPersonCharacter_C|SetoCartAtHand Player 0)
  (Transformation|DetachFromComponent (Variables|Default|GetCartdidgeColl) "KeepRelative" "KeepRelative" "KeepWorld" true)
  (Physics|SetSimulatePhysics (Variables|Default|GetCartdidgeColl) true)
  (Variables|Default|SetbIsHeld false))