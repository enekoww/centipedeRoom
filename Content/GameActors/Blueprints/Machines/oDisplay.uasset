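; oDisplay is the console room's television, an interactable that toggles the in-room game on and off.
; It registers with gmConsoleRoom on BeginPlay; OnActivate calls NewGame, showing the camera-render material and score widget only when the console holds a cartridge, otherwise static noise.
; Activating again during play restores static, hides the widget and destroys the grid system.
; An overlap area toggles an info text for the first-person character.
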(event OnComponentBeginOverlap(AreaOfIntereaction)
  (params (OverlappedComponent :type Primitive%20Component%20Object%20Reference) (OtherActor :type Actor%20Object%20Reference) (OtherComp :type Primitive%20Component%20Object%20Reference) (OtherBodyIndex :type Integer) (bFromSweep :type Boolean) (SweepResult :type Hit%20Result%20Structure%20%28by%20ref%29))
  ;[1 1 1] Set information billboard visibility
  (Utilities|Casting|CastToFirstPersonCharacter OtherActor)
  (Rendering|SetVisibility (Variables|Default|GetTextRender) true false))

(event OnComponentEndOverlap(AreaOfIntereaction)
  (params (OverlappedComponent :type Primitive%20Component%20Object%20Reference) (OtherActor :type Actor%20Object%20Reference) (OtherComp :type Primitive%20Component%20Object%20Reference) (OtherBodyIndex :type Integer))
  ;[1 1 1] Set information billboard visibility
  (Utilities|Casting|CastToFirstPersonCharacter OtherActor)
  (Rendering|SetVisibility (Variables|Default|GetTextRender) false false))

(event EventBeginPlay
  ;[1 1 1] Set relevant variables. Hide widget.
  (Rendering|Material|SetMaterial (Variables|Default|GetTv) 0 "/Game/GameActors/Blueprints/Machines/Materials/mStaticNoise_Mat.mStaticNoise_Mat")
  (bind _asgm_console_room (Utilities|Casting|CastTogmConsoleRoom (Game|GetGameMode)))
  (Variables|/Game/GameActors/Blueprints/gmConsoleRoom.gmConsoleRoom_C|SetoTelevision _asgm_console_room self)
  (Rendering|SetVisibility (Variables|Default|GetPointSystem) false false))

(event Collision|EventActorBeginOverlap
  (params (OtherActor :type Actor%20Object%20Reference)))

(event EventTick
  (params (DeltaSeconds :type Float%20%28single-precision%29)))

(event EventOnActivate
  ;[1 1 1] Handle interface call. If conditions met game starts. Posses Centipede, fix game camera
  (if (Variables|Default|GetbIsGaming)
    (CallFunction|OnDeactivate)
    (else
      (bind _asgm_console_room (Utilities|Casting|CastTogmConsoleRoom (Game|GetGameMode)))
      (Utilities|IsValid (Variables|/Game/GameActors/Blueprints/Machines/oConsole.oConsole_C|GetoGameCartIn (Variables|/Game/GameActors/Blueprints/gmConsoleRoom.gmConsoleRoom_C|GetoConsole _asgm_console_room))
        (:Is%20Valid
          ;;[1 1 1] Render Camera to Material
          (Rendering|Material|SetMaterial (Variables|Default|GetTv) 0 "/Game/Camera/cameraFrustrum_Mat.cameraFrustrum_Mat")
          (Default|NewGame _asgm_console_room)
          (Variables|Default|SetbIsGaming true)
          (Rendering|SetVisibility (Variables|Default|GetPointSystem) true false)
          (Rendering|SetVisibility (Variables|Default|GetTextRender) false false))
        (:Is%20Not%20Valid
          (Rendering|Material|SetMaterial (Variables|Default|GetTv) 0 "/Game/GameActors/Blueprints/Machines/Materials/mStaticNoise_Mat.mStaticNoise_Mat")
          (Default|NewGame _asgm_console_room)
          (Rendering|SetVisibility (Variables|Default|GetPointSystem) false false))))))

(event EventOnDeactivate
  ;[1 1 1] Turn off console and deactivate game. Posses Player again
  (Rendering|Material|SetMaterial (Variables|Default|GetTv) 0 "/Game/GameActors/Blueprints/Machines/Materials/mStaticNoise_Mat.mStaticNoise_Mat")
  (bind _asgm_console_room (Utilities|Casting|CastTogmConsoleRoom (Game|GetGameMode)))
  (Default|AutoDestroy (Variables|/Game/GameActors/Blueprints/gmConsoleRoom.gmConsoleRoom_C|GetoGridSystem _asgm_console_room))
  (Actor|DestroyActor (Variables|/Game/GameActors/Blueprints/gmConsoleRoom.gmConsoleRoom_C|GetoGridSystem _asgm_console_room))
  (Variables|Default|SetbIsGaming false)
  (Rendering|SetVisibility (Variables|Default|GetPointSystem) false false))

(fn ConstructionScript)