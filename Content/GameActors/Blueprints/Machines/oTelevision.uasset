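; Television machine in the console room that shows static noise when idle and registers itself with the gmConsoleRoom game mode on BeginPlay.
; Activating it toggles play: with a cartridge in the console, it switches the screen to the CameraFrustrum material and starts a new game.
; Without a cartridge it keeps static but still calls NewGame.
; Deactivating restores static and destroys the game mode's grid system.
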(event EventBeginPlay
  (Rendering|Material|SetMaterial (Variables|Default|GetTv) 0 "/Game/GameActors/Blueprints/Machines/mStaticNoise.mStaticNoise")
  (bind _asgm_console_room (Utilities|Casting|CastTogmConsoleRoom (Game|GetGameMode)))
  (Variables|/Game/GameActors/Blueprints/gmConsoleRoom.gmConsoleRoom_C|SetoTelevision _asgm_console_room self))

(event Collision|EventActorBeginOverlap
  (params (OtherActor :type Actor%20Object%20Reference)))

(event EventTick
  (params (DeltaSeconds :type Float%20%28single-precision%29)))

(event EventOnActivate
  (bind _tv (Variables|Default|GetTv))
  (if (Variables|Default|GetbIsGaming)
    (CallFunction|OnDeactivate)
    (else
      (bind _asgm_console_room (Utilities|Casting|CastTogmConsoleRoom (Game|GetGameMode)))
      (Utilities|IsValid (Variables|/Game/GameActors/Blueprints/Machines/oConsole.oConsole_C|GetoGameCartIn (Variables|/Game/GameActors/Blueprints/gmConsoleRoom.gmConsoleRoom_C|GetoConsole _asgm_console_room))
        (:Is%20Valid
          (Rendering|Material|SetMaterial _tv 0 "/Game/Camera/cameraFrustrum_Mat.cameraFrustrum_Mat")
          (Default|NewGame _asgm_console_room)
          (Variables|Default|SetbIsGaming true))
        (:Is%20Not%20Valid
          (Rendering|Material|SetMaterial _tv 0 "/Game/GameActors/Blueprints/Machines/mStaticNoise.mStaticNoise")
          (Default|NewGame _asgm_console_room))))))

(event EventOnDeactivate
  (Rendering|Material|SetMaterial (Variables|Default|GetTv) 0 "/Game/GameActors/Blueprints/Machines/mStaticNoise.mStaticNoise")
  (bind _asgm_console_room (Utilities|Casting|CastTogmConsoleRoom (Game|GetGameMode)))
  (Default|AutoDestroy (Variables|/Game/GameActors/Blueprints/gmConsoleRoom.gmConsoleRoom_C|GetoGridSystem _asgm_console_room))
  (Actor|DestroyActor (Variables|/Game/GameActors/Blueprints/gmConsoleRoom.gmConsoleRoom_C|GetoGridSystem _asgm_console_room))
  (Variables|Default|SetbIsGaming false))

(fn ConstructionScript)