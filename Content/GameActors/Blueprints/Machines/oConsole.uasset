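; oConsole is a game console machine in the console room that accepts and ejects game cartridges when activated.
; It registers itself with gmConsoleRoom, and inserting moves the player's held cartridge onto the socket with collision disabled.
; Activating a loaded console either swaps in the held cartridge or, if the player holds none, ejects and calls NewGame on the game mode.
; Ejected cartridges regain physics and get a randomized launch impulse.
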(event Custom|InsertCart
  (bind _asfirst_person_character (Utilities|Casting|CastToFirstPersonCharacter (Game|Player|GetPlayerPawn 0)))
  (Utilities|IsValid (Variables|/Game/GameActors/Blueprints/FirstPersonCharacter.FirstPersonCharacter_C|GetoCartAtHand _asfirst_person_character)
    (:Is%20Valid
      (bind _output_get (Variables|Default|SetoGameCartIn (Variables|/Game/GameActors/Blueprints/FirstPersonCharacter.FirstPersonCharacter_C|GetoCartAtHand _asfirst_person_character)))
      (Collision|SetCollisionEnabled (Variables|/Game/GameActors/Blueprints/Machines/oGridCartdridge.oGridCartdridge_C|GetCartdidgeColl _output_get) "NoCollision")
      (Transformation|AttachComponentToComponent (Variables|/Game/GameActors/Blueprints/Machines/oGridCartdridge.oGridCartdridge_C|GetCartdidgeColl (Variables|/Game/GameActors/Blueprints/FirstPersonCharacter.FirstPersonCharacter_C|GetoCartAtHand _asfirst_person_character)) (Variables|Default|GetCartdridgeSocket) "CartdridgeSocket" "SnapToTarget" "SnapToTarget" "KeepWorld" true)
      (Variables|/Game/GameActors/Blueprints/FirstPersonCharacter.FirstPersonCharacter_C|SetoCartAtHand _asfirst_person_character 0))))

(event Custom|EjectCart
  (Collision|SetCollisionEnabled (Variables|/Game/GameActors/Blueprints/Machines/oGridCartdridge.oGridCartdridge_C|GetCartdidgeColl (Variables|Default|GetoGameCartIn)) "QueryAndPhysics")
  (Transformation|DetachFromActor (Variables|Default|GetoGameCartIn) "KeepRelative" "KeepRelative" "KeepWorld")
  (Physics|SetSimulatePhysics (Variables|/Game/GameActors/Blueprints/Machines/oGridCartdridge.oGridCartdridge_C|GetCartdidgeColl (Variables|Default|GetoGameCartIn)) true)
  (Physics|AddImpulse (Variables|/Game/GameActors/Blueprints/Machines/oGridCartdridge.oGridCartdridge_C|GetCartdidgeColl (Variables|Default|GetoGameCartIn)) (Math|Vector|MakeVector (Math|Conversions|ToFloat(Integer) (Math|Random|RandomIntegerinRange -3000 3000)) (Math|Conversions|ToFloat(Integer) (Math|Random|RandomIntegerinRange 1000 3000)) 5e+03) "None" false)
  (Variables|Default|SetoGameCartIn 0))

(event Collision|EventActorBeginOverlap
  (params (OtherActor :type Actor%20Object%20Reference)))

(event EventTick
  (params (DeltaSeconds :type Float%20%28single-precision%29)))

(event EventOnActivate
  (Utilities|IsValid (Variables|Default|GetoGameCartIn)
    (:Is%20Valid
      (bind _holding (CallFunction|PlayerHoldingCart))
      (if _holding
        (CallFunction|EjectCart)
        (CallFunction|InsertCart)
        (else
          (CallFunction|EjectCart)
          (bind _asgm_console_room (Utilities|Casting|CastTogmConsoleRoom (Game|GetGameMode)))
          (Default|NewGame _asgm_console_room))))
    (:Is%20Not%20Valid
      (CallFunction|InsertCart))))

(event EventBeginPlay
  (bind _asgm_console_room (Utilities|Casting|CastTogmConsoleRoom (Game|GetGameMode)))
  (Variables|/Game/GameActors/Blueprints/gmConsoleRoom.gmConsoleRoom_C|SetoConsole _asgm_console_room self))

(fn ConstructionScript)

(fn PlayerHoldingCart
  (bind _asfirst_person_character (Utilities|Casting|CastToFirstPersonCharacter (Game|Player|GetPlayerPawn 0)))
  (Utilities|IsValid (Variables|/Game/GameActors/Blueprints/FirstPersonCharacter.FirstPersonCharacter_C|GetoCartAtHand _asfirst_person_character)
    (:Is%20Valid
      (return true))
    (:Is%20Not%20Valid
      (return false))))