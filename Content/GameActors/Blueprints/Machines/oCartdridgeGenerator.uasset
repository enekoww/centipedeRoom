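; A machine actor that spawns an OGridCartdridge 50 units above itself when activated.
; An interaction area toggles a prompt's visibility as the first-person character enters and leaves.
; While the player is inside, a looping timer yaws the prompt toward them, avoiding Tick, and is cleared on exit.
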(event OnComponentBeginOverlap(AreaOfInteraction)
  (params (OverlappedComponent :type Primitive%20Component%20Object%20Reference) (OtherActor :type Actor%20Object%20Reference) (OtherComp :type Primitive%20Component%20Object%20Reference) (OtherBodyIndex :type Integer) (bFromSweep :type Boolean) (SweepResult :type Hit%20Result%20Structure%20%28by%20ref%29))
  (bind _asfirst_person_character (Utilities|Casting|CastToFirstPersonCharacter OtherActor))
  (Variables|Default|SetPlayer _asfirst_person_character)
  (bind _returnvalue (Utilities|Time|SetTimerbyFunctionName 0 "LookAtPlayerText" 0.05 true))
  (Variables|Default|SetLookAtTimer _returnvalue)
  (Rendering|ToggleVisibility (Variables|Default|GetPrompt) false))

(event OnComponentEndOverlap(AreaOfInteraction)
  (params (OverlappedComponent :type Primitive%20Component%20Object%20Reference) (OtherActor :type Actor%20Object%20Reference) (OtherComp :type Primitive%20Component%20Object%20Reference) (OtherBodyIndex :type Integer))
  (if (== OtherActor (Variables|Default|GetPlayer))
    (Variables|Default|SetPlayer 0)
    (Utilities|Time|ClearandInvalidateTimerbyHandle (Variables|Default|GetLookAtTimer))
    (Rendering|ToggleVisibility (Variables|Default|GetPrompt) false)))

(event EventBeginPlay)

(event Collision|EventActorBeginOverlap
  (params (OtherActor :type Actor%20Object%20Reference)))

(event EventTick
  (params (DeltaSeconds :type Float%20%28single-precision%29)))

(event EventOnActivate
  (bind _returnvalue (Transformation|GetActorTransform))
  (Game|SpawnActorfromClass "/Game/GameActors/Blueprints/Machines/oGridCartdridge.oGridCartdridge_C" (Math|Transform|MakeTransform (+ (.location _returnvalue) "0, 0,50.000000") (.rotation _returnvalue) (.scale _returnvalue)) "Undefined" 0 20 20 1e+01 0.3 0 0))

(fn ConstructionScript)

(fn LookatPlayerText
  (Transformation|SetWorldRotation (Variables|Default|GetPrompt) (Math|Rotator|MakeRotator 0.0 0.0 (.yaw (Math|Rotator|FindLookatRotation (Transformation|GetActorLocation) (Transformation|GetActorLocation (Variables|Default|GetPlayer))))) false false))