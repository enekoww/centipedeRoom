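; Grid tile actor that, on impact, turns into a temporary vertical wall of blocking tiles.
; CreateWall walks the same grid column from the actor's tile toward the maximum Y, blocking each empty tile and starting its clean-up timer.
; Impact then frees the actor's own tile, swaps the cube material and destroys the actor after a brief delay.
; A separate OnPoints event spawns a points actor at the tile with the destroy score.
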(event EventBeginPlay
  (|CallParentFunction) ; This node is disabled and will not be called.\nDrag off pins to build functionality.
)

(event Collision|EventActorBeginOverlap
  (params (OtherActor :type Actor%20Object%20Reference)))

(event EventTick
  (params (DeltaSeconds :type Float%20%28single-precision%29)))

(event EventOnPoints
  (Game|SpawnActorfromClass "/Game/Widgets/aPointsSpawn.aPointsSpawn_C" (Transformation|GetActorTransform (Variables|Default|GetoGridTileReference)) "Undefined" 0 (Variables|Default|GetiDestroyPoints) 0))

(event EventOnImpact
  (bind _ogridtilereference (Variables|Default|GetoGridTileReference))
  (Utilities|IsValid _ogridtilereference
    (:Is%20Valid
      (CallFunction|CreateWall _ogridtilereference)
      (Variables|/Game/GameActors/Blueprints/Grid/oGridTile.oGridTile_C|SetoActorOnTile _ogridtilereference 0)
      (Variables|/Game/GameActors/Blueprints/Grid/oGridTile.oGridTile_C|SetfIsBlocking _ogridtilereference false)
      (Rendering|Material|SetMaterial (Variables|Default|Getcube) 0 "/Engine/EngineMaterials/CubeMaterial.CubeMaterial")
      (Utilities|FlowControl|RetriggerableDelay 0.1)
      (Actor|DestroyActor))))

(fn ConstructionScript
  (|CallParentFunction))

(fn CreateWall
  (params (ReferenceTIle :type O%20Grid%20Tile%20Object%20Reference))
  (bind _v2dgridposition (Variables|/Game/GameActors/Blueprints/Grid/oGridTile.oGridTile_C|Getv2dGridPosition ReferenceTIle))
  (bind _ogridsystem (Variables|Default|GetoGridSystem))
  (for _index (range (Math|Float|Truncate (.y _v2dgridposition)) (Variables|/Game/GameActors/Blueprints/Grid/oGridSystem.oGridSystem_C|GetiYCellNumber _ogridsystem))
    (Utilities|IsValid (.Value (Utilities|Map|Find (Variables|/Game/GameActors/Blueprints/Grid/oGridSystem.oGridSystem_C|GetmGridArray _ogridsystem) (Math|Vector2D|MakeVector2D (.x _v2dgridposition) (Math|Conversions|ToFloat(Integer) _index))))
      (:Is%20Valid
        (Utilities|IsValid (Variables|/Game/GameActors/Blueprints/Grid/oGridTile.oGridTile_C|GetoActorOnTile (.Value (Utilities|Map|Find (Variables|/Game/GameActors/Blueprints/Grid/oGridSystem.oGridSystem_C|GetmGridArray _ogridsystem) (Math|Vector2D|MakeVector2D (.x _v2dgridposition) (Math|Conversions|ToFloat(Integer) _index)))))
          (:Is%20Not%20Valid
            (Default|MakeBlocking (.Value (Utilities|Map|Find (Variables|/Game/GameActors/Blueprints/Grid/oGridSystem.oGridSystem_C|GetmGridArray _ogridsystem) (Math|Vector2D|MakeVector2D (.x _v2dgridposition) (Math|Conversions|ToFloat(Integer) _index)))) (.Value (Utilities|Map|Find (Variables|/Game/GameActors/Blueprints/Grid/oGridSystem.oGridSystem_C|GetmGridArray _ogridsystem) (Math|Vector2D|MakeVector2D (.x _v2dgridposition) (Math|Conversions|ToFloat(Integer) _index)))))
            (Default|SetCleanTileTimer (.Value (Utilities|Map|Find (Variables|/Game/GameActors/Blueprints/Grid/oGridSystem.oGridSystem_C|GetmGridArray _ogridsystem) (Math|Vector2D|MakeVector2D (.x _v2dgridposition) (Math|Conversions|ToFloat(Integer) _index)))))))))))