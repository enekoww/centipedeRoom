(event Custom|ResetDoOnce
  (bind _oobstacle (Variables|Default|GetoObstacle))
  ;[1 1 1] On Kill Tile
  (Utilities|FlowControl|DoOnce false) ; enters at Reset
)

(event Custom|SetCleanTileTimer
  ;[1 1 1] Clean TIle after X seconds
  (Utilities|FlowControl|RetriggerableDelay 4.0)
  (bind _asobstacle (Utilities|Casting|CastToObstacle (Variables|Default|GetoObstacle)))
  (Utilities|IsValid _asobstacle
    (:Is%20Valid
      (Rendering|Material|SetMaterial (Variables|/Game/GameActors/Blueprints/Grid/Obstacle.Obstacle_C|Getcube _asobstacle) 0 "/DatasmithContent/Materials/FBXImporter/VREDMaster.VREDMaster")
      (Utilities|FlowControl|Delay 1.0)
      (CallFunction|MakeNonBlocking))))

(event Collision|EventActorBeginOverlap
  (params (OtherActor :type Actor%20Object%20Reference)))

(event EventOnImpact)

(event EventBeginPlay
  ;[1 1 1] Initialize
  (bind _aso_grid_system (Utilities|Casting|CastTooGridSystem (Components|GetOwner)))
  (Variables|Default|SetoGridSystem _aso_grid_system)
  (Variables|Default|SetvGridWorldLocation (Transformation|GetActorLocation))
  (bind _asgm_console_room (Utilities|Casting|CastTogmConsoleRoom (Game|GetGameMode)))
  (Variables|Default|SetgmConsoleRoom _asgm_console_room))

(event EventOnKill
  (bind _oobstacle (Variables|Default|GetoObstacle))
  ;[1 1 1] On Kill Tile
  (Utilities|FlowControl|DoOnce false
    (:Completed
      (Utilities|IsValid _oobstacle
        (:Is%20Valid
          (Default|OnImpact _oobstacle)
          (Default|OnPoints _oobstacle))))))

(fn ConstructionScript
  (Variables|Default|SetfBoxSize (Variables|Default|GetfBoxSize)))

(fn MakeBlocking
  (params (CurrentTile :type O%20Grid%20Tile%20Object%20Reference))
  (Utilities|IsValid CurrentTile
    (:Is%20Valid
      (Variables|OwnerBooleans|SetfIsBlocking true)
      (bind _returnvalue (Game|SpawnActorfromClass "/Game/GameActors/Blueprints/Grid/Obstacle.Obstacle_C" (Transformation|GetActorTransform) "Undefined" (Variables|Default|GetoGridSystem) self 0))
      (bind _output_get (Variables|Default|SetoObstacle _returnvalue))
      (Utilities|IsValid _output_get
        (:Is%20Valid
          (Variables|/Game/GameActors/Blueprints/Grid/Obstacle.Obstacle_C|SetoGridTileReference _returnvalue CurrentTile)
          (Variables|Default|SetoActorOnTile _returnvalue)
          (return _returnvalue))
        (:Is%20Not%20Valid
          (Development|PrintString "not valid opn spawbn"))))
    (:Is%20Not%20Valid
      (Development|PrintString "failed"))))

(fn MakeNonBlocking
  (bind _oactorontile (Variables|Default|GetoActorOnTile))
  (Variables|OwnerBooleans|SetfIsBlocking false)
  (Utilities|IsValid _oactorontile
    (:Is%20Valid
      (Actor|DestroyActor _oactorontile))))

(fn MakeBoundary
  (params (CurrentTile :type O%20Grid%20Tile%20Object%20Reference))
  (Variables|OwnerBooleans|SetfIsBlocking true)
  (bind _returnvalue (Game|SpawnActorfromClass "/Game/GameActors/Blueprints/Grid/Bounding.Bounding_C" (Transformation|GetActorTransform) "Undefined" (Variables|Default|GetoGridSystem) 0 0))
  (bind _output_get (Variables|Default|SetoObstacle _returnvalue))
  (Variables|/Game/GameActors/Blueprints/Grid/Obstacle.Obstacle_C|SetoGridTileReference _returnvalue CurrentTile)
  (Variables|OwnerBooleans|SetbIsBoundary true)
  (return _output_get))

(fn GivePoints
  (Game|SpawnActorfromClass "/Game/Widgets/aPointsSpawn.aPointsSpawn_C" (Transformation|GetActorTransform) "Undefined" 0 (Variables|Default|GetiPointsForDestroying) 0))

(fn MakeBlockingSpecial
  (params (CurrentTile :type O%20Grid%20Tile%20Object%20Reference) (ToSpawnSpecial :type eObstacleTypes%20Enum%20%28by%20ref%29 :default "NewEnumerator0"))
  (Utilities|IsValid CurrentTile
    (:Is%20Valid
      (Variables|OwnerBooleans|SetfIsBlocking true)
      (bind _obstacle (CallFunction|MakSpecialObstacle ToSpawnSpecial))
      (bind _output_get (Variables|Default|SetoObstacle _obstacle))
      (Utilities|IsValid _output_get
        (:Is%20Valid
          (Variables|/Game/GameActors/Blueprints/Grid/Obstacle.Obstacle_C|SetoGridTileReference _obstacle CurrentTile)
          (Variables|Default|SetoActorOnTile _obstacle)
          (return _obstacle))
        (:Is%20Not%20Valid
          (Development|PrintString "not valid opn spawbn"))))))

(fn MakeObstacle
  (bind _returnvalue (Game|SpawnActorfromClass "/Game/GameActors/Blueprints/Grid/Obstacle.Obstacle_C" (Transformation|GetActorTransform) "Undefined" (Variables|Default|GetoGridSystem) self 0))
  (return _returnvalue))

(fn MakeBarrel
  (bind _returnvalue (Game|SpawnActorfromClass "/Game/GameActors/Blueprints/Grid/oBarrel.oBarrel_C" (Transformation|GetActorTransform) "Undefined" (Variables|Default|GetoGridSystem) self 0))
  (return _returnvalue))

(fn MakeHorizontalWall
  (bind _returnvalue (Game|SpawnActorfromClass "/Game/GameActors/Blueprints/Grid/oHorizontalWall.oHorizontalWall_C" (Transformation|GetActorTransform) "Undefined" (Variables|Default|GetoGridSystem) self 0))
  (return _returnvalue))

(fn MakeVertWall
  (bind _returnvalue (Game|SpawnActorfromClass "/Game/GameActors/Blueprints/Grid/oVerticalWall.oVerticalWall_C" (Transformation|GetActorTransform) "Undefined" (Variables|Default|GetoGridSystem) self 0))
  (return _returnvalue))

(fn MakSpecialObstacle
  (params (NewParam :type eObstacleTypes%20Enum :default "NewEnumerator0"))
  (switch Utilities|FlowControl|Switch|SwitchoneObstacleTypes NewParam
    (:NewEnumerator0
      (bind _newparam (CallFunction|MakeObstacle))
      (return _newparam))
    (:NewEnumerator1
      (bind _newparam_2 (CallFunction|MakeBarrel))
      (return _newparam_2))
    (:NewEnumerator2
      (bind _newparam_3 (CallFunction|MakeHorizontalWall))
      (return _newparam_3))
    (:NewEnumerator3
      (bind _newparam_4 (CallFunction|MakeVertWall))
      (return _newparam_4))))