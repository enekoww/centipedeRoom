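; Grid actor that, on impact, turns into a horizontal wall of blocking tiles.
; CreateWall looks up three tiles centered on its X in the adjacent +Y row through the grid system's map, and calls MakeBlocking on those without an actor.
; The impact then frees its own tile, swaps the cube material and destroys the actor after a brief delay.
; A separate OnPoints event spawns a points actor at the tile.
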(event EventBeginPlay
  (|CallParentFunction) ; This node is disabled and will not be called.\nDrag off pins to build functionality.
)

(event Collision|EventActorBeginOverlap
  (params (OtherActor :type Actor%20Object%20Reference)))

(event EventTick
  (params (DeltaSeconds :type Float%20%28single-precision%29)))

(event EventOnPoints
  (Game|SpawnActorfromClass "/Game/Widgets/aPointsSpawn.aPointsSpawn_C" (Transformation|GetActorTransform (Variables|Default|GetoGridTileReference)) "Undefined" 0 (Variables|Default|GetiDestroyPoints) 0))

(event EventOnImpact
  (bind _ogridtilereference (Variables|Default|GetoGridTileReference))
  (Utilities|IsValid _ogridtilereference
    (:Is%20Valid
      (CallFunction|CreateWall _ogridtilereference)
      (Variables|/Game/GameActors/Blueprints/Grid/oGridTile.oGridTile_C|SetoActorOnTile _ogridtilereference 0)
      (Variables|/Game/GameActors/Blueprints/Grid/oGridTile.oGridTile_C|SetfIsBlocking _ogridtilereference false)
      (Rendering|Material|SetMaterial (Variables|Default|Getcube) 0 "/Engine/EngineMaterials/CubeMaterial.CubeMaterial")
      (Utilities|FlowControl|RetriggerableDelay 0.1)
      (Actor|DestroyActor))))

(fn ConstructionScript
  (|CallParentFunction))

(fn CreateWall
  (params (ReferenceTIle :type O%20Grid%20Tile%20Object%20Reference))
  (bind _returnvalue (Math|Vector2D|MakeVector2D -1.0 1.0))
  (bind _v2dgridposition (Variables|/Game/GameActors/Blueprints/Grid/oGridTile.oGridTile_C|Getv2dGridPosition ReferenceTIle))
  (bind _returnvalue_2 (+ _v2dgridposition _returnvalue))
  (bind _returnvalue_3 (Math|Float|Truncate (.x _returnvalue_2)))
  (for _index (range _returnvalue_3 (+ _returnvalue_3 2))
    (Utilities|IsValid (Variables|/Game/GameActors/Blueprints/Grid/oGridTile.oGridTile_C|GetoActorOnTile (.Value (Utilities|Map|Find (Variables|/Game/GameActors/Blueprints/Grid/oGridSystem.oGridSystem_C|GetmGridArray (Variables|Default|GetoGridSystem)) (Math|Vector2D|MakeVector2D (Math|Conversions|ToFloat(Integer) _index) (.y _returnvalue_2)))))
      (:Is%20Not%20Valid
        (Default|MakeBlocking (.Value (Utilities|Map|Find (Variables|/Game/GameActors/Blueprints/Grid/oGridSystem.oGridSystem_C|GetmGridArray (Variables|Default|GetoGridSystem)) (Math|Vector2D|MakeVector2D (Math|Conversions|ToFloat(Integer) _index) (.y _returnvalue_2)))) (.Value (Utilities|Map|Find (Variables|/Game/GameActors/Blueprints/Grid/oGridSystem.oGridSystem_C|GetmGridArray (Variables|Default|GetoGridSystem)) (Math|Vector2D|MakeVector2D (Math|Conversions|ToFloat(Integer) _index) (.y _returnvalue_2)))))))))