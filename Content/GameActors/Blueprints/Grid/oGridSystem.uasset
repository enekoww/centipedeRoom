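; Grid actor for a Centipede-style game that builds the playfield of tiles and populates it with obstacles.
; On BeginPlay it spawns OGridTile actors into a map keyed by 2D grid position, turning side columns into boundaries and random valid tiles into starting obstacles.
; A looping timer then randomly adds obstacles within weighted depth bands, using neighbour checks to avoid diagonals.
; AutoDestroy clears tiles, obstacles, centipede parts, shooters and projectiles.
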(event Custom|SetupFirstGame
  (Utilities|FlowControl|Sequence
    (:then_0
      (CallFunction|GenerateGrid))
    (:then_1
      ;[1 1 1] Sends delegate to GameMode and cretes New Centipede
      (Utilities|FlowControl|Delay 0.2))))

(event Custom|RandomObstacleGenerator
  ;[1 1 1] Runtime Obstacle Generator Timer
  (bind _returnvalue (Utilities|Time|SetTimerbyFunctionName 0 "AddRandomObstacleToGrid" (Variables|Default|GetfObstacleGeneratorLoopTime) true))
  (Variables|Default|SetObstacleTimer _returnvalue))

(event Custom|RandomObstacleGeneratorStop
  ;[1 1 1] Runtime Obstacle Generator Timer
  (Utilities|Time|ClearandInvalidateTimerbyHandle (Variables|Default|GetObstacleTimer)))

(event Custom|Generate%20Grid
  (bind _ftilehalfextent (Variables|Tile|GetfTileHalfExtent))
  (Utilities|FlowControl|Sequence
    (:then_0
      ;[1 1 1] GidSystem Definition
      (Variables|Grid|SetiGridSize (* (Variables|Grid|GetiXCellNumber) (Variables|Grid|GetiYCellNumber)))
      (for _index (range 0 (- (Variables|Grid|GetiXCellNumber) 1))
        (Variables|Tile|SetiXIndex _index)
        (for _index_2 (range 0 (- (Variables|Grid|GetiYCellNumber) 1))
          (Variables|Tile|SetiYIndex _index_2)
          ;[1 1 1] GridTile Definition
          (bind _transform (CallFunction|CalculateTransform))
          (bind _returnvalue (Game|SpawnActorfromClass "/Game/GameActors/Blueprints/Grid/oGridTile.oGridTile_C" _transform "Undefined" self 0))
          (bind _output_get (Variables|Tile|SetoCurrentTile _returnvalue))
          (CallFunction|SetPositionVector _output_get)
          (Components|Box|SetBoxExtent (Variables|/Game/GameActors/Blueprints/Grid/oGridTile.oGridTile_C|GetBox (Variables|Tile|GetoCurrentTile)) (Math|Vector|MakeVector _ftilehalfextent _ftilehalfextent 0.0) true)
          ;[1 1 1] Tile Map with Pos Vector as Key
          (Utilities|Map|Add (Variables|Default|GetmGridArray) (Variables|Tile|Getv2dCurrentVector) (Variables|Tile|GetoCurrentTile)))))
    (:then_1
      ;[1 1 1] Start Putting Obstacles
      (CallFunction|SetBlockignTilesEvent))))

(event Custom|SetBlockignTilesEvent
  (bind _acandidatetoblocktiles (Variables|Default|GetaCandidateToBlockTiles))
  (bind _returnvalue (Utilities|Array|Length _acandidatetoblocktiles))
  (bind _returnvalue_2 (- _returnvalue 1))
  (bind _returnvalue_3 (Math|Random|RandomInteger _returnvalue_2))
  (bind _output (Utilities|Array|Get(acopy) _acandidatetoblocktiles _returnvalue_3))
  ;[1 1 1] Set Obstacles
  (bind _values (Utilities|Map|Values (Variables|Default|GetmGridArray)))
  (for _array_element _values
    (bind _isboundary (CallFunction|IsBoundary _array_element))
    (if _isboundary
      ;;[1 1 1] Generate Boundaries
      (bind _obstacle (Default|MakeBoundary _array_element _array_element))
      (Utilities|IsValid _obstacle
        (:Is%20Valid
          (Variables|/Game/GameActors/Blueprints/Grid/Obstacle.Obstacle_C|SetbIsBoundary _obstacle true)))
      (else
        ;;[1 1 1] Get Obstacle all Candidates
        (bind _validtile (CallFunction|IsObstaclePosValid _array_element))
        (if _validtile
          (Utilities|Array|AddUnique (Variables|Default|GetaCandidateToBlockTiles) _array_element)))))
  ;;[1 1 1] Randomly Choose Initial Obstacle Population
  (for _index (range 0 (- (Variables|Default|GetiInitialBlocks) 1))
    (bind _obstacle_2 (Default|MakeBlocking _output _output))
    (Utilities|IsValid _obstacle_2
      (:Is%20Valid
        (Variables|/Game/GameActors/Blueprints/Grid/Obstacle.Obstacle_C|SetbIsBoundary _obstacle_2 false))))
  ;;[1 1 1] Start Runtime Obstacle Generator
  (CallFunction|RandomObstacleGenerator))

(event Custom|AutoDestroy
  ;[1 1 1] Destroy This Grid And Actors Inside
  (CallFunction|DestroyAll))

(event EventBeginPlay
  (CallFunction|SetupFirstGame))

(event Collision|EventActorBeginOverlap
  (params (OtherActor :type Actor%20Object%20Reference)))

(fn ConstructionScript
  (Variables|Grid|SetiXCellNumber (Variables|Grid|GetiXCellNumber))
  (Variables|Grid|SetiYCellNumber (Variables|Grid|GetiYCellNumber))
  (Variables|Tile|SetfTileHalfExtent (Variables|Tile|GetfTileHalfExtent))
  (bind _outactors (Actor|GetAllActorsOfClass "/Game/Camera/SceneCaptureCam.SceneCaptureCam_C"))
  (CallFunction|SetGridCenteredPosition (+ (Transformation|GetActorLocation (Utilities|Array|Get(acopy) _outactors)) "0, 0,300.000000")))

(fn GetTilePosition
  (params (vTileNumer :type Vector%202D%20Structure))
  (bind _mgridarray (Variables|Default|GetmGridArray))
  (bind (_value _returnvalue) (Utilities|Map|Find _mgridarray vTileNumer))
  ;[1 1 1] Return World Location of Tile
  (if _returnvalue
    (return (Transformation|GetActorLocation _value))))

(fn IsObstaclePosValid
  (params (CurrentGrid :type O%20Grid%20Tile%20Object%20Reference))
  (bind _output_get (LocalVariables|SetCurrentTile CurrentGrid))
  (if (not (Variables|/Game/GameActors/Blueprints/Grid/oGridTile.oGridTile_C|GetfIsBlocking _output_get))
    (if (or (== (.y (Variables|/Game/GameActors/Blueprints/Grid/oGridTile.oGridTile_C|Getv2dGridPosition (LocalVariables|GetCurrentTile))) 0.0) (>= (.y (Variables|/Game/GameActors/Blueprints/Grid/oGridTile.oGridTile_C|Getv2dGridPosition (LocalVariables|GetCurrentTile))) (Math|Conversions|ToFloat(Integer) (- (Variables|Grid|GetiYCellNumber) 2))))
      _
      (else
        (Utilities|IsValid (.Value (Utilities|Map|Find (Variables|Default|GetmGridArray) (- (Variables|/Game/GameActors/Blueprints/Grid/oGridTile.oGridTile_C|Getv2dGridPosition (LocalVariables|GetCurrentTile)) 1.0)))
          (:Is%20Valid
            (Utilities|IsValid (.Value (Utilities|Map|Find (Variables|Default|GetmGridArray) (Math|Vector2D|MakeVector2D (+ (.x (Variables|/Game/GameActors/Blueprints/Grid/oGridTile.oGridTile_C|Getv2dGridPosition (LocalVariables|GetCurrentTile))) -1.0) (+ (.y (Variables|/Game/GameActors/Blueprints/Grid/oGridTile.oGridTile_C|Getv2dGridPosition (LocalVariables|GetCurrentTile))) 1.0))))
              (:Is%20Valid
                (if (or (Variables|/Game/GameActors/Blueprints/Grid/oGridTile.oGridTile_C|GetfIsBlocking (.Value (Utilities|Map|Find (Variables|Default|GetmGridArray) (- (Variables|/Game/GameActors/Blueprints/Grid/oGridTile.oGridTile_C|Getv2dGridPosition (LocalVariables|GetCurrentTile)) 1.0)))) (Variables|/Game/GameActors/Blueprints/Grid/oGridTile.oGridTile_C|GetfIsBlocking (.Value (Utilities|Map|Find (Variables|Default|GetmGridArray) (Math|Vector2D|MakeVector2D (+ (.x (Variables|/Game/GameActors/Blueprints/Grid/oGridTile.oGridTile_C|Getv2dGridPosition (LocalVariables|GetCurrentTile))) -1.0) (+ (.y (Variables|/Game/GameActors/Blueprints/Grid/oGridTile.oGridTile_C|Getv2dGridPosition (LocalVariables|GetCurrentTile))) 1.0))))))
                  _
                  (else
                    (return true)))))))))
    (return false)))

(fn IsBoundary
  (params (NewParam1 :type O%20Grid%20Tile%20Object%20Reference))
  (bind _v2dgridposition (Variables|/Game/GameActors/Blueprints/Grid/oGridTile.oGridTile_C|Getv2dGridPosition NewParam1))
  (return (or (== (.x _v2dgridposition) 0.0) (== (.x _v2dgridposition) (Math|Conversions|ToFloat(Integer) (- (Variables|Grid|GetiXCellNumber) 1))))))

(fn AddRandomObstacletoGrid
  (bind _iycellnumber (Variables|Grid|GetiYCellNumber))
  (bind _possiblelocations (LocalVariables|GetPossibleLocations))
  (bind _mgridarray (Variables|Default|GetmGridArray))
  (bind _returnvalue (Utilities|Array|Length _possiblelocations))
  (bind _returnvalue_2 (Math|Random|RandomIntegerinRange 0 _returnvalue))
  (bind _output (Utilities|Array|Get(acopy) _possiblelocations _returnvalue_2))
  (bind _value (Utilities|Map|Find _mgridarray _output))
  ;[1 1 1] Throw Dice to chance of making blocking
  (if (>= (Math|Random|RandomFloat) 0.4)
    ;[1 1 1] Set Limits
    (if (<= (Math|Random|RandomFloat) (LocalVariables|GetbChanceOfLowOnGrid))
      (LocalVariables|SetiMinDepth (Math|Float|Truncate (* _iycellnumber 0.66)))
      (LocalVariables|SetiMaxDepth (- _iycellnumber 2))
      (else
        (LocalVariables|SetiMinDepth 2)
        (LocalVariables|SetiMaxDepth (Math|Float|Truncate (* (Variables|Grid|GetiYCellNumber) 0.66)))))
    ;[1 1 1] Get All Candidates
    (bind _keys (Utilities|Map|Keys (Variables|Default|GetmGridArray)))
    (for _array_element _keys
      (bind _output_get (LocalVariables|Setv2dVector (Math|Vector2D|MakeVector2D (.x _array_element) (.y _array_element))))
      (if (and (>= (Math|Float|Truncate (.y _array_element)) (LocalVariables|GetiMinDepth)) (<= (Math|Float|Truncate (.y _array_element)) (LocalVariables|GetiMaxDepth)))
        (bind _validtile (CallFunction|IsObstaclePosValid (.Value (Utilities|Map|Find (Variables|Default|GetmGridArray) _output_get))))
        (if _validtile
          (Utilities|Array|AddUnique (LocalVariables|GetPossibleLocations) (LocalVariables|Getv2dVector)))))
    ;[1 1 1] Make Blocking over Chance
    (if (not (Variables|/Game/GameActors/Blueprints/Grid/oGridTile.oGridTile_C|GetfIsBlocking _value))
      (Default|MakeBlocking _value _value))))

(fn DestroyAll
  (bind _outactors (Actor|GetAllActorsOfClass "/Game/GameActors/Blueprints/Characters/Player/pCentipedeHead.pCentipedeHead_C"))
  (Utilities|IsValid (Utilities|Array|Get(acopy) _outactors)
    (:Is%20Valid
      (Actor|DestroyActor (Utilities|Array|Get(acopy) _outactors)))
    (:Is%20Not%20Valid
      _))
  (bind _values (Utilities|Map|Values (Variables|Default|GetmGridArray)))
  (for _array_element _values
    (Actor|DestroyActor _array_element))
  (bind _outactors_2 (Actor|GetAllActorsOfClass "/Game/GameActors/Blueprints/Grid/Obstacle.Obstacle_C"))
  (for _array_element_2 _outactors_2
    (Actor|DestroyActor _array_element_2))
  (bind _outactors_3 (Actor|GetAllActorsOfClass "/Game/GameActors/Blueprints/Characters/Enemy/aShooter.aShooter_C"))
  (for _array_element_3 _outactors_3
    (Actor|DestroyActor _array_element_3))
  (bind _outactors_4 (Actor|GetAllActorsOfClass "/Game/GameActors/Blueprints/Characters/Enemy/aProjectile.aProjectile_C"))
  (for _array_element_4 _outactors_4
    (Actor|DestroyActor _array_element_4))
  (bind _outactors_5 (Actor|GetAllActorsOfClass "/Game/GameActors/Blueprints/Characters/Player/centipedeTail.centipedeTail_C"))
  (for _array_element_5 _outactors_5
    (Actor|DestroyActor _array_element_5)))

(fn CalculateTransform
  ;[1 1 1] Calculate Position of Tile Based on Size
  (bind _correctedposition (CallFunction|SetGridCenteredPosition (Variables|Default|GetvDesiredLocation)))
  (return (Math|Transform|MakeTransform (Math|Vector|MakeVector (.x (- _correctedposition (Math|Vector|MakeVector (* (Math|Conversions|ToFloat(Integer) (Variables|Tile|GetiXIndex)) (* 2 (Variables|Tile|GetfTileHalfExtent))) (* (Math|Conversions|ToFloat(Integer) (Variables|Tile|GetiYIndex)) (* 2 (Variables|Tile|GetfTileHalfExtent))) 0.0))) (.y (- _correctedposition (Math|Vector|MakeVector (* (Math|Conversions|ToFloat(Integer) (Variables|Tile|GetiXIndex)) (* 2 (Variables|Tile|GetfTileHalfExtent))) (* (Math|Conversions|ToFloat(Integer) (Variables|Tile|GetiYIndex)) (* 2 (Variables|Tile|GetfTileHalfExtent))) 0.0))) 1.8e+02))))

(fn SetPositionVector
  (params (Current%20Tile :type O%20Grid%20Tile%20Object%20Reference))
  (bind _output_get (Variables|/Game/GameActors/Blueprints/Grid/oGridTile.oGridTile_C|Setv2dGridPosition Current%20Tile (Math|Vector2D|MakeVector2D (Math|Conversions|ToFloat(Integer) (Variables|Tile|GetiXIndex)) (Math|Conversions|ToFloat(Integer) (Variables|Tile|GetiYIndex)))))
  (Variables|Tile|Setv2dCurrentVector _output_get))

(fn SetGridCenteredPosition
  (params (DesiredCenterPosition :type Vector))
  (return (Math|Vector|MakeVector (+ (.x DesiredCenterPosition) (/ (* (Variables|Grid|GetiXCellNumber) (* (Variables|Tile|GetfTileHalfExtent) 2.0)) 2.0)) (+ (.y DesiredCenterPosition) (/ (* (Variables|Grid|GetiYCellNumber) (* (Variables|Tile|GetfTileHalfExtent) 2.0)) 2.0)) (.z DesiredCenterPosition))))