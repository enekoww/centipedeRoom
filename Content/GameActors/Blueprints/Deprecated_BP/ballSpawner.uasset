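; Deprecated ball spawner actor that endlessly drops FirstPersonProjectile actors from its location, starting on BeginPlay.
; SpawnBall places each projectile at a random world Y offset around the actor, aimed along its negated up vector.
; It then calls the Wait event, which delays a short random whole number of seconds and calls SpawnBall again, forming the loop without Tick.
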(event Custom|Wait
  (Utilities|FlowControl|Delay (Math|Conversions|ToFloat(Integer) (Math|Random|RandomIntegerinRange 1 2)))
  (CallFunction|SpawnBall))

(event EventBeginPlay
  (CallFunction|SpawnBall))

(event Collision|EventActorBeginOverlap
  (params (OtherActor :type Actor%20Object%20Reference)))

(event EventTick
  (params (DeltaSeconds :type Float%20%28single-precision%29)))

(fn ConstructionScript)

(fn SpawnBall
  (bind _returnvalue (Transformation|GetActorTransform))
  (Game|SpawnActorfromClass "/Game/GameActors/Blueprints/Deprecated_BP/FirstPersonProjectile.FirstPersonProjectile_C" (Math|Transform|MakeTransform (Math|Vector|MakeVector (.x (.location _returnvalue)) (+ (.y (.location _returnvalue)) (Math|Conversions|ToFloat(Integer) (Math|Random|RandomIntegerinRange -300 300))) (.z (.location _returnvalue))) (Math|Conversions|RotationFromXVector (* (Transformation|GetActorUpVector) -1.0)) (.scale _returnvalue)) "Undefined" 0 0)
  (CallFunction|Wait))